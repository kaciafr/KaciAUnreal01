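; Player telekinesis (gravity gun) ability that attracts or ejects physics objects using Fire and AltFire.
; Input events run a macro chain: camera-relative points, visibility trace, grab target update with damping save/restore, then force calculation.
; Force pulls toward a hold point or pushes toward the ray end, scaled by distance-based curves.
; It applies mostly at the body, partly at the impact point, with high damping while attracting.
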(event Input|EnhancedActionEvents|EnhancedInputActionIA_Debug1
  (params (ActionValue :type Boolean) (ElapsedSeconds :type Float%20%28double-precision%29) (TriggeredSeconds :type Float%20%28double-precision%29) (InputAction :type Input%20Action%20Object%20Reference :default "/Game/Core/Input/Actions/IA_Debug1.IA_Debug1"))
  (:Started
    (Development|PrintString "GravityGun Started"))
  (:Completed
    (Development|PrintString "GravityGun Completed")))

(event Input|EnhancedActionEvents|EnhancedInputActionIA_Fire
  (params (ActionValue :type Boolean) (ElapsedSeconds :type Float%20%28double-precision%29) (TriggeredSeconds :type Float%20%28double-precision%29) (InputAction :type Input%20Action%20Object%20Reference :default "/Game/Core/Input/Actions/IA_Fire.IA_Fire"))
  (:Triggered
    (Variables|Default|SetbIsAttracting true)
    (|CalcPoints :!label _label)
    (|RayCast)
    (|InitGrabbed
      (:execute
        (|CalcForce
          (:OutputPin
            (|ApplyForce
              (:then
                _)
              (:OutputPin
                _))
            (Rendering|Debug|DrawDebugSphere (Variables|Default|GetRayOrigin) 1.0 12 "(R=0.085301,G=1.000000,B=0.000000,A=1.000000)" 5.0)
            (Rendering|Debug|DrawDebugSphere (Variables|Default|GetDestination) 1.0 12 "(R=1.000000,G=0.000000,B=0.065137,A=1.000000)" 5.0))))))
  (:Canceled
    (Variables|Default|SetbIsAttracting false :!label _label_2)
    (goto _label))
  (:Completed
    (goto _label_2)))

(event Input|EnhancedActionEvents|EnhancedInputActionIA_AltFire
  (params (ActionValue :type Boolean) (ElapsedSeconds :type Float%20%28double-precision%29) (TriggeredSeconds :type Float%20%28double-precision%29) (InputAction :type Input%20Action%20Object%20Reference :default "/Game/Core/Input/Actions/IA_AltFire.IA_AltFire"))
  (:Triggered
    (Variables|Default|SetbIsEjecting true)
    (|CalcPoints :!label _label)
    (|RayCast)
    (|InitGrabbed
      (:execute
        (|CalcForce
          (:OutputPin
            (|ApplyForce
              (:then
                _)
              (:OutputPin
                _))
            (Rendering|Debug|DrawDebugSphere (Variables|Default|GetRayOrigin) 1.0 12 "(R=0.085301,G=1.000000,B=0.000000,A=1.000000)" 5.0)
            (Rendering|Debug|DrawDebugSphere (Variables|Default|GetDestination) 1.0 12 "(R=1.000000,G=0.000000,B=0.065137,A=1.000000)" 5.0))))))
  (:Canceled
    (Variables|Default|SetbIsEjecting false :!label _label_2)
    (goto _label))
  (:Completed
    (goto _label_2)))

(event EventBeginPlay
  ;[0.15 0.15 0.15 0.5] Init Character
  (bind _asbp_character (Utilities|Casting|CastToBP_Character (Components|GetOwner)))
  (Variables|Default|SetCharacter_0 _asbp_character))

(fn OldGetPoints
  (bind _camera (Utilities|GetCamera))
  (bind _returnvalue (Transformation|GetWorldTransform _camera))
  (Variables|Default|SetRayOrigin (Math|Transform|TransformLocation _returnvalue (Math|Vector|MakeVector 0.0 0.0 0.0)))
  (Variables|Default|SetRayEnd (Math|Transform|TransformLocation _returnvalue (Math|Vector|MakeVector (Variables|Default|GetRayDistance) 0.0 0.0)))
  (Variables|Default|SetDestination (Math|Transform|TransformLocation _returnvalue (Variables|Default|GetDestinationLocal)))
  (return (Variables|Default|GetRayOrigin) (Variables|Default|GetRayEnd) (Variables|Default|GetDestination)))

(fn OldRayCast
  (params (Start :type Vector) (End :type Vector))
  (bind (_outhit _returnvalue) (Collision|LineTraceByChannel Start End "TraceTypeQuery1" false 0 "ForOneFrame" true "(R=1.000000,G=0.000000,B=0.000000,A=1.000000)" "(R=0.000000,G=1.000000,B=0.000000,A=1.000000)" 2.0))
  (if _returnvalue
    (Variables|Default|SetImpact (.ImpactPoint (Collision|BreakHitResult _outhit)))
    (bind _asprimitive_component (Utilities|Casting|CastToPrimitiveComponent (Variables|/Script/Engine.Actor|GetRootComponent (.HitActor (Collision|BreakHitResult _outhit))))
      (:then
        _)
      (:CastFailed
        _))
    (else
      (Variables|Default|SetImpact (Variables|Default|GetRayEnd))))
  (return (Physics|IsSimulatingPhysics _asprimitive_component "None")))

(fn OIldSetGrabbedObject
  (params (NextGrabbedObject :type Primitive%20Component%20Object%20Reference))
  (if (== NextGrabbedObject (Variables|Default|GetGrabbed))
    _
    (else
      (if (Utilities|IsValid (Variables|Default|GetGrabbed))
        (Class|PrimitiveComponent|SetLinearDamping (Variables|Default|GetGrabbed) (Variables|Default|GetInitLinearDamping))
        (Class|PrimitiveComponent|SetAngularDamping (Variables|Default|GetGrabbed) (Variables|Default|GetInitAngularDamping)))
      (Variables|Default|SetGrabbed NextGrabbedObject)
      (if (Utilities|IsValid NextGrabbedObject)
        (Variables|Default|SetInitLinearDamping (Class|PrimitiveComponent|GetLinearDamping NextGrabbedObject))
        (Variables|Default|SetInitAngularDamping (Class|PrimitiveComponent|GetAngularDamping NextGrabbedObject)))))
  (return))
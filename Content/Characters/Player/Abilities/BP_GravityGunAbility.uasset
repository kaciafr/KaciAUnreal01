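; Gravity gun ability component for the player character that pushes or pulls physics objects under the camera's aim.
; While the charged or combo attack input is held, Tick line-traces from the camera on the Visibility channel.
; A hit actor with a physics-simulating root receives force at the impact point along the view direction.
; IsGrab flips the force's sign: charged attack applies Force as set, combo attack negates it.
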(event Input|EnhancedActionEvents|EnhancedInputActionIA_Debug1
  (params (ActionValue :type Boolean) (ElapsedSeconds :type Float%20%28double-precision%29) (TriggeredSeconds :type Float%20%28double-precision%29) (InputAction :type Input%20Action%20Object%20Reference :default "/Game/Core/Input/Actions/IA_Debug1.IA_Debug1"))
  (:Started
    (Development|PrintString "GravityGun Started"))
  (:Completed
    (Development|PrintString "GravityGun Completed")))

(event Input|EnhancedActionEvents|EnhancedInputActionIA_ChargedAttack
  (params (ActionValue :type Boolean) (ElapsedSeconds :type Float%20%28double-precision%29) (TriggeredSeconds :type Float%20%28double-precision%29) (InputAction :type Input%20Action%20Object%20Reference :default "/Game/Variant_Combat/Input/Actions/IA_ChargedAttack.IA_ChargedAttack"))
  (:Started
    (Variables|Default|SetbIsGrab true)
    (Variables|Default|SetbIsActivated true))
  (:Completed
    (Variables|Default|SetbIsActivated false)))

(event Input|EnhancedActionEvents|EnhancedInputActionIA_ComboAttack
  (params (ActionValue :type Boolean) (ElapsedSeconds :type Float%20%28double-precision%29) (TriggeredSeconds :type Float%20%28double-precision%29) (InputAction :type Input%20Action%20Object%20Reference :default "/Game/Variant_Combat/Input/Actions/IA_ComboAttack.IA_ComboAttack"))
  (:Started
    (Variables|Default|SetbIsGrab false)
    (Variables|Default|SetbIsActivated true))
  (:Completed
    (Variables|Default|SetbIsActivated false)))

(event EventBeginPlay
  ;[0.15 0.15 0.15 0.5] Init Character
  (bind _asbp_character (Utilities|Casting|CastToBP_Character (Components|GetOwner)))
  (Variables|Default|SetCharacter _asbp_character))

(event EventTick
  (params (DeltaSeconds :type Float%20%28single-precision%29))
  (bind _camera (Utilities|GetCamera))
  (bind _force (Variables|Default|GetForce))
  ;[0.15 0.15 0.15 0.5] Init Direction And Start
  (if (Variables|Default|GetbIsActivated)
    (Variables|Default|SetDirection (Math|Vector|GetForwardVector _camera))
    (bind _output_get (Variables|Default|SetStart (Transformation|GetWorldLocation _camera)))
    ;[0.15 0.15 0.15 0.5] RayCast Target
    (bind (_outhit _returnvalue) (Collision|LineTraceByChannel _output_get (+ _output_get (* (Variables|Default|GetDirection) (Variables|Default|GetDistance))) "TraceTypeQuery1" false 0 "None" true "(R=1.000000,G=0.000000,B=0.000000,A=1.000000)" "(R=0.000000,G=1.000000,B=0.000000,A=1.000000)" 2.0))
    (if _returnvalue
      (Variables|Default|SetImpactPoint (.ImpactPoint (Collision|BreakHitResult _outhit)))
      (bind _asprimitive_component (Utilities|Casting|CastToPrimitiveComponent (Variables|/Script/Engine.Actor|GetRootComponent (.HitActor (Collision|BreakHitResult _outhit)))))
      (if (Physics|IsSimulatingPhysics _asprimitive_component "None")
        (Variables|Default|SetTarget _asprimitive_component)
        ;[0.15 0.15 0.15 0.5] Apply Force
        (Class|PrimitiveComponent|AddForceatLocation (Variables|Default|GetTarget) (* (Variables|Default|GetDirection) (Math|Float|SelectFloat _force (- 0.0 _force) (Variables|Default|GetbIsGrab))) (Variables|Default|GetImpactPoint) "None")))))
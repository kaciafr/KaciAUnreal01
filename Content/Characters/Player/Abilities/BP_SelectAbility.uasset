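; Player ability selector component that tracks which of its owner's abilities is active.
; On BeginPlay it gathers the owner's BP_AbilityBase components into RegisteredAbilities, printing each added index for debugging.
; The O and P keys each pick a fixed index, setting ActiveAbility both through OnAbilityInputPressed and by a redundant direct SetActiveAbility call.
; It only selects the ability and does not activate it, and the array lookup has no bounds check.
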(event Custom|OnAbilityInputPressed
  (params (AbilityIndex :type Integer))
  (CallFunction|SetActiveAbility AbilityIndex))

(event EventBeginPlay
  (for _array_element (Actor|GetComponentsByClass (Components|GetOwner) "/Game/Characters/Player/Abilities/BP_AbilityBase.BP_AbilityBase_C")
    (bind _asbp_ability_base (Utilities|Casting|CastToBP_AbilityBase _array_element))
    (bind _returnvalue (Utilities|Array|Add (Variables|Default|GetRegisteredAbilities) _asbp_ability_base))
    (Development|PrintString (Utilities|String|ToString(Integer) _returnvalue) true true "(R=0.000000,G=0.660000,B=1.000000,A=1.000000)" 1e+01)))

(event Input|KeyboardEvents|O
  (params (Key :type Key%20Structure :default "None"))
  (:Pressed
    (CallFunction|OnAbilityInputPressed 1)
    (CallFunction|SetActiveAbility 1)))

(event Input|KeyboardEvents|P
  (params (Key :type Key%20Structure :default "None"))
  (:Pressed
    (CallFunction|OnAbilityInputPressed)
    (CallFunction|SetActiveAbility)))

(fn SetActiveAbility
  (params (AbilityIndex :type Integer))
  (Variables|Default|SetActiveAbility (Utilities|Array|Get(acopy) (Variables|Default|GetRegisteredAbilities) AbilityIndex)))
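; Base class for player abilities, providing shared helpers that work on the owning BP_Character.
; It finds or adds components on the character and exposes its camera, HP, Mana and Stamina.
; Mana and Stamina helpers forward consume and drain calls to the resource objects.
; A camera-forward trace targets PhysicsBody objects with debug drawing, and keyed Log helpers print debug values on screen.
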(event EventBeginPlay)

(event EventTick
  (params (DeltaSeconds :type Float%20%28single-precision%29)))

(fn GetorCreateComponent
  (params (Class :type Actor%20Component%20Class%20Reference))
  (bind _character (CallFunction|GetCharacter))
  (if (Utilities|IsValid (Actor|GetComponentbyClass _character Class))
    (return (Actor|GetComponentbyClass _character Class) false)
    (else
      (bind _returnvalue (Game|AddComponentbyClass _character Class))
      (return _returnvalue true))))

(fn GetCharacter
  (bind _asbp_character (Utilities|Casting|CastToBP_Character (Components|GetOwner))
    (:then
      (return _asbp_character))
    (:CastFailed
      (Development|PrintString "Cast to Character error" true true "(R=1.000000,G=0.000000,B=0.000000,A=1.000000)"))))

(fn GetCamera
  (bind _character (CallFunction|GetCharacter))
  (if (Utilities|IsValid (Variables|/Game/Characters/Player/BP_Character.BP_Character_C|GetCamera _character))
    (return (Variables|/Game/Characters/Player/BP_Character.BP_Character_C|GetCamera _character) (Transformation|GetWorldTransform (Variables|/Game/Characters/Player/BP_Character.BP_Character_C|GetCamera _character)))
    (else
      (Development|PrintString "No Camera on Character" true true "(R=1.000000,G=0.000000,B=0.000000,A=1.000000)"))))

(fn GetCameraPoint
  (params (Forward :type Float%20%28double-precision%29) (Left :type Float%20%28double-precision%29) (Up :type Float%20%28double-precision%29))
  (bind _camera (CallFunction|GetCamera))
  (return (Math|Transform|TransformLocation (Transformation|GetWorldTransform _camera) (Math|Vector|MakeVector Forward Left Up))))

(fn CameraLineTrace
  (params (MaxDistance :type Float%20%28double-precision%29))
  (bind _camera (CallFunction|GetCamera))
  (LocalVariables|Set_RayStart (Math|Transform|TransformLocation (Transformation|GetWorldTransform _camera) (Math|Vector|MakeVector 0.0 0.0 0.0)))
  (LocalVariables|Set_RayEnd (Math|Transform|TransformLocation (Transformation|GetWorldTransform _camera) (Math|Vector|MakeVector MaxDistance 0.0 0.0)))
  (bind (_outhit _returnvalue) (Collision|LineTraceForObjects (Math|Transform|TransformLocation (Transformation|GetWorldTransform _camera) (Math|Vector|MakeVector 0.0 0.0 0.0)) (Math|Transform|TransformLocation (Transformation|GetWorldTransform _camera) (Math|Vector|MakeVector MaxDistance 0.0 0.0)) (Utilities|Array|MakeArray "ObjectTypeQuery4") false 0 "ForDuration" true "(R=1.000000,G=0.000000,B=0.000000,A=1.000000)" "(R=0.000000,G=1.000000,B=0.000000,A=1.000000)" 2.0))
  (LocalVariables|Set_Hit _outhit)
  (bind _output_get (LocalVariables|Set_IsHit _returnvalue))
  (if _output_get
    (LocalVariables|Set_HitImpact (.ImpactPoint (Collision|BreakHitResult (LocalVariables|Get_Hit))))
    (bind _asprimitive_component (Utilities|Casting|CastToPrimitiveComponent (Variables|/Script/Engine.Actor|GetRootComponent (.HitActor (Collision|BreakHitResult (LocalVariables|Get_Hit)))))
      (:then
        (LocalVariables|Set_HitPrimitive _asprimitive_component))
      (:CastFailed
        (return (LocalVariables|Get_RayStart) (LocalVariables|Get_RayEnd) (LocalVariables|Get_IsHit) (Physics|IsSimulatingPhysics _asprimitive_component "None") (LocalVariables|Get_Hit) (LocalVariables|Get_HitImpact) (LocalVariables|Get_HitPrimitive) (.Distance (Collision|BreakHitResult (LocalVariables|Get_Hit))))))
    (else
      (LocalVariables|Set_HitImpact (LocalVariables|Get_RayEnd))
      (return (LocalVariables|Get_RayStart) (LocalVariables|Get_RayEnd) (LocalVariables|Get_IsHit) (Physics|IsSimulatingPhysics _asprimitive_component "None") (LocalVariables|Get_Hit) (LocalVariables|Get_HitImpact) (LocalVariables|Get_HitPrimitive) (.Distance (Collision|BreakHitResult (LocalVariables|Get_Hit)))))))

(fn LogString
  (params (Name :type String) (Value :type String) (Color :type Linear%20Color%20Structure :default "(R=1.000000,G=0.000000,B=1.000000,A=1.000000)") (Duration :type Float%20%28single-precision%29))
  (Development|PrintString (Utilities|String|Append Name ": " Value) true true Color Duration (Utilities|String|StringToName Name))
  (return))

(fn LogBoolean
  (params (Name :type String) (Value :type Boolean) (True :type Linear%20Color%20Structure :default "(R=0.000000,G=1.000000,B=0.000000,A=1.000000)") (False :type Linear%20Color%20Structure :default "(R=1.000000,G=0.000000,B=0.000000,A=1.000000)"))
  (CallFunction|LogString Name (Utilities|String|ToString(Integer) (Math|Conversions|ToInteger(Boolean) Value)) (select Value True False) 5.0)
  (return))

(fn LogFloat
  (params (Name :type String) (Value :type Float%20%28double-precision%29) (Color :type Linear%20Color%20Structure :default "(R=0.500000,G=1.000000,B=0.000000,A=1.000000)") (Duration :type Float%20%28single-precision%29))
  (CallFunction|LogString Name (Utilities|String|ToString(Float) Value) Color Duration)
  (return))

(fn LogVector
  (params (Name :type String) (Value :type Vector) (Color :type Linear%20Color%20Structure :default "(R=1.000000,G=1.000000,B=0.000000,A=1.000000)") (Duration :type Float%20%28single-precision%29))
  (CallFunction|LogString Name (Utilities|String|ToString(Vector) Value) Color Duration)
  (return))

(fn GetMana
  (bind _character (CallFunction|GetCharacter))
  (return (Variables|/Game/Characters/Player/BP_Character.BP_Character_C|GetMana _character) (Variables|/Game/Characters/Player/BP_Resource.BP_Resource_C|GetCurrentValue (Variables|/Game/Characters/Player/BP_Character.BP_Character_C|GetMana _character))))

(fn GetHP
  (bind _character (CallFunction|GetCharacter))
  (return (Variables|/Game/Characters/Player/BP_Character.BP_Character_C|GetHP _character) (Variables|/Game/Characters/Player/BP_Resource.BP_Resource_C|GetCurrentValue (Variables|/Game/Characters/Player/BP_Character.BP_Character_C|GetHP _character))))

(fn GetStamina
  (bind _character (CallFunction|GetCharacter))
  (return (Variables|/Game/Characters/Player/BP_Character.BP_Character_C|GetStamina _character) (Variables|/Game/Characters/Player/BP_Resource.BP_Resource_C|GetCurrentValue (Variables|/Game/Characters/Player/BP_Character.BP_Character_C|GetStamina _character))))

(fn ConsumeStamina
  (params (Amount :type Float%20%28double-precision%29))
  (bind _staminaresource (CallFunction|GetStamina))
  (bind _success (Default|Consume _staminaresource Amount))
  (return _success))

(fn ConsumeMana
  (params (Amount :type Float%20%28double-precision%29))
  (bind _manaresource (CallFunction|GetMana))
  (bind _success (Default|Consume _manaresource Amount))
  (return _success))

(fn DrainStamina
  (params (DrainRate :type Float%20%28double-precision%29))
  (bind _staminaresource (CallFunction|GetStamina))
  (bind _success (Default|Drain _staminaresource DrainRate))
  (return _success))

(fn DrainMana
  (params (DrainRate :type Float%20%28double-precision%29))
  (bind _manaresource (CallFunction|GetMana))
  (bind _success (Default|Drain _manaresource DrainRate))
  (return _success))
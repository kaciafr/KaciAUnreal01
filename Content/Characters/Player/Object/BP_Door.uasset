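; BP_Door is a puzzle door that opens when its candles are lit in the correct order.
; It binds to each candle's change event at BeginPlay and appends the array index of each newly lit candle to a password string.
; A prefix check against the correct password resets all candles on a wrong step.
; A full match calls OpenDoor, which shifts the two door meshes apart instantly.
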(event Custom|OnCandleChanged
  (params (Sender :type BP%20Caddle%20Object%20Reference) (bIsLit :type Boolean))
  (if bIsLit
    (bind _output_get (Variables|Default|SetCurrentPassword (Utilities|String|Append (Variables|Default|GetCurrentPassword) (Utilities|String|ToString(Integer) (Utilities|Array|FindItem (Variables|Default|GetCandleArray) Sender)))))
    (if (Utilities|String|StartsWith (Variables|Default|GetCorrectPassword) _output_get)
      (if (Utilities|Enum|Equal(Enum) (Variables|Default|GetCurrentPassword) (Variables|Default|GetCorrectPassword))
        (CallFunction|OpenDoor)
        (Default|Reset (Variables|Default|GetCandleArray)))
      (else
        (for _array_element (Variables|Default|GetCandleArray)
          (Default|Reset _array_element)
          (Variables|Default|SetCurrentPassword ""))))))

(event EventBeginPlay
  (for _array_element (Variables|Default|GetCandleArray)
    (EventDispatchers|BindEventtoOnChanged _array_element (delegate Custom|OnCandleChanged))))

(event Collision|EventActorBeginOverlap
  (params (OtherActor :type Actor%20Object%20Reference)))

(event EventTick
  (params (DeltaSeconds :type Float%20%28single-precision%29)))

(fn ConstructionScript)

(fn OpenDoor
  (Variables|Default|SetisOpen true)
  (Utilities|FlowControl|Sequence
    (:then_0
      (Transformation|AddRelativeLocation (Variables|Default|GetDoormesh) "-100.000000,0.000000,0.000000" false false))
    (:then_1
      (Transformation|AddRelativeLocation (Variables|Default|GetDoormesh1) "100.000000,0.000000,0.000000" false false))))
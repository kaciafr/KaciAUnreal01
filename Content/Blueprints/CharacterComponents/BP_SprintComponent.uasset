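; Character component that lets BP_Character sprint while the sprint input is held, at a stamina cost.
; On BeginPlay it caches the owning character and its BP_StaminaComponent, then applies normal speed.
; Each IA_Sprint trigger asks the stamina component to consume stamina per second, setting MaxWalkSpeed to sprint speed on success and normal speed otherwise.
; Releasing the input restores normal speed.
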(event Input|EnhancedActionEvents|EnhancedInputActionIA_Sprint
  (params (ActionValue :type Boolean) (ElapsedSeconds :type Float%20%28double-precision%29) (TriggeredSeconds :type Float%20%28double-precision%29) (InputAction :type Input%20Action%20Object%20Reference :default "/Game/Input/Actions/IA_Sprint.IA_Sprint"))
  (:Triggered
    (bind _success (Default|ConsumeStaminaPerSecond (Variables|Default|GetBP_StaminaComponent) (Variables|Default|GetStaminaCostPerSecond)))
    (if _success
      (CallFunction|SetSpeed (Variables|Default|GetSprintSpeed))
      (else
        (CallFunction|ResetSpeed))))
  (:Completed
    (CallFunction|ResetSpeed)))

(event EventBeginPlay
  (bind _asbp_character (Utilities|Casting|CastToBP_Character (Components|GetOwner)))
  (Variables|Default|SetBP_Character _asbp_character)
  (Variables|Default|SetBP_StaminaComponent (Actor|GetComponentbyClass _asbp_character "/Game/Blueprints/CharacterComponents/BP_StaminaComponent.BP_StaminaComponent_C"))
  (CallFunction|ResetSpeed))

(event EventTick
  (params (DeltaSeconds :type Float%20%28single-precision%29)))

(fn ResetSpeed
  (CallFunction|SetSpeed (Variables|Default|GetNormalSpeed)))

(fn SetSpeed
  (params (MaxWalkSpeed :type Float%20%28single-precision%29))
  (Variables|/Script/Engine.CharacterMovementComponent|SetMaxWalkSpeed (Variables|/Script/Engine.Character|GetCharacterMovement (Variables|Default|GetBP_Character)) MaxWalkSpeed))
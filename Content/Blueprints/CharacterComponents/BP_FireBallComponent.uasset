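; Character component that lets its owner cast a fireball from the IA_FireBall input action.
; A CanShoot flag and a cooldown delay limit how often the input can trigger a shot.
; Each shot plays a montage on the owning Character, then after a fixed delay rather than an anim notify spawns BP_FireBall just ahead of the actor, oriented along its control rotation.
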(event Custom|ShootFireBall
  (bind _returnvalue (Components|GetOwner))
  (bind _ascharacter (Utilities|Casting|CastToCharacter _returnvalue))
  (Animation|PlayAnimMontage _ascharacter "/Game/Anim/AM_Character.AM_Character" 1.0 "None")
  (Utilities|FlowControl|Delay 2.5)
  (Game|SpawnActorfromClass "/Game/Blueprints/BP_FireBall.BP_FireBall_C" (Math|Transform|MakeTransform (+ (* (Math|Vector|GetForwardVector (Pawn|GetControlRotation _ascharacter :!class /Script/Engine.Pawn)) 1e+02) (Transformation|GetActorLocation _returnvalue)) (Pawn|GetControlRotation _ascharacter :!class /Script/Engine.Pawn)) "Undefined" "MultiplyWithRoot" 0 0))

(event Input|EnhancedActionEvents|EnhancedInputActionIA_FireBall
  (params (ActionValue :type Boolean) (ElapsedSeconds :type Float%20%28double-precision%29) (TriggeredSeconds :type Float%20%28double-precision%29) (InputAction :type Input%20Action%20Object%20Reference :default "/Game/Variant_Combat/Input/Actions/IA_FireBall.IA_FireBall"))
  (:Started
    (if (Variables|Default|GetCanShoot)
      (CallFunction|ShootFireBall)
      (Variables|Default|SetCanShoot false)
      (Utilities|FlowControl|Delay (Variables|Default|GetCouldown))
      (Variables|Default|SetCanShoot true))))

(event EventBeginPlay)

(event EventTick
  (params (DeltaSeconds :type Float%20%28single-precision%29)))
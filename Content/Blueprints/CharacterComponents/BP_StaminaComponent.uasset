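; Character component that tracks a stamina pool, starting full at Max on BeginPlay.
; ConsumeStamina spends an amount only if enough remains, returns whether it succeeded, and pushes the next regen time back by RegenDelay.
; Tick regenerates stamina at RegenRate up to Max once that delay has passed, printing the value on screen as a debug readout while regenerating.
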(event EventBeginPlay
  (Variables|Default|SetStamina (Variables|Default|GetMax)))

(event EventTick
  (params (DeltaSeconds :type Float%20%28single-precision%29))
  (if (CallFunction|CanRegen)
    (bind _output_get (Variables|Default|SetStamina (Math|Float|Clamp(Float) (+ (Variables|Default|GetStamina) (* (Variables|Default|GetRegenRate) DeltaSeconds)) 0.0 (Variables|Default|GetMax))))
    (Development|PrintString (Utilities|String|ToString(Float) _output_get) true true "(R=1.000000,G=0.000000,B=0.971976,A=1.000000)" 2.0 "stamina")))

(fn ConsumeStamina
  (params (Amount :type Float%20%28double-precision%29))
  (if (< (- (Variables|Default|GetStamina) Amount) 0.0)
    (return false)
    (else
      (Variables|Default|SetStamina (- (Variables|Default|GetStamina) Amount))
      (Variables|Default|SetNextRegenTime (+ (Variables|Default|GetRegenDelay) (Utilities|Time|GetTimeSeconds)))
      (return true))))

(fn CanRegen
  (return (< (Variables|Default|GetNextRegenTime) (Utilities|Time|GetTimeSeconds))))
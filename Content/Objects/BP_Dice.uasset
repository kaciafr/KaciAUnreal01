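; BP_Dice is a colorable die actor whose physics can be rigged toward a target face value.
; Each tick it looks up TargetFaceValue in CheatRotations and offsets the mesh's center of mass by the scaled result, weighting the die.
; The construction script calls SetColor, which stores the color and applies it to the mesh materials.
; An unconnected torque-correction experiment with debug prints remains in the event graph.
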(event EventBeginPlay)

(event Collision|EventActorBeginOverlap
  (params (OtherActor :type Actor%20Object%20Reference)))

(event EventTick
  (params (DeltaSeconds :type Float%20%28single-precision%29))
  (bind _targetfacevalue (Variables|Default|GetTargetFaceValue))
  (bind _cheatrotations (Variables|Default|GetCheatRotations))
  (bind (_value _returnvalue) (Utilities|Map|Find _cheatrotations _targetfacevalue))
  (if _returnvalue
    (Class|PrimitiveComponent|SetCenterOfMass (Variables|Default|GetDiceMesh) (* _value 1.2e+02) "None")))

(fn ConstructionScript
  (CallFunction|SetColor (Variables|Default|GetColor)))

(fn SetColor
  (params (Color :type Color%20Structure))
  (bind _output_get (Variables|Default|SetColor Color))
  (Rendering|Material|SetColorParameterValueonMaterials (Variables|Default|GetDiceMesh) "BaseColorFactor" (Math|Conversions|ToLinearColor(Color) _output_get))
  (return))